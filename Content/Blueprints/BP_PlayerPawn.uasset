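; BP_PlayerPawn is an unfinished player pawn Blueprint with input-driven movement and bullet firing sketched out but not wired.
; Its axis, BeginPlay and overlap events are empty, so none of the logic runs.
; Disconnected nodes would store axis values, call OnFire, spawn BP_Bullet at a world transform, and move the actor by normalized direction, Speed0 and delta time.
; The direction vector is still zero, unlinked to the stored inputs.
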(event EventBeginPlay)

(event Collision|EventActorBeginOverlap
  (params (OtherActor :type Actor%20Object%20Reference)))

(event Input|ActionEvents|InputActionFire
  (params (Key :type Key%20Structure :default "None")))

(event Input|AxisEvents|InputAxisHorizontal
  (params (AxisValue :type Float%20%28single-precision%29)))

(event Input|AxisEvents|InputAxisVertical
  (params (AxisValue :type Float%20%28single-precision%29)))

(fn ConstructionScript)
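; BP_Tail is an actor sketched to chase the player pawn, but its logic is disconnected, so it does nothing at runtime.
; BeginPlay, Tick and the construction script are empty.
; An orphaned branch would cache the player pawn as Target0, which a comment says is meant to happen at spawn.
; An unused expression computes a frame-rate-independent step toward Target0 at Speed0, while the unreached SetActorLocation targets the world origin.
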(event EventBeginPlay
  ;[0 0 0] 태어날 때 PlayerPawn을 목적지로 삼는다.
)

(event Collision|EventActorBeginOverlap
  (params (OtherActor :type Actor%20Object%20Reference)))

(event EventTick
  (params (DeltaSeconds :type Float%20%28single-precision%29)))

(fn ConstructionScript)